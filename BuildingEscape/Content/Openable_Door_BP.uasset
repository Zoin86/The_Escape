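; Openable door Blueprint that swings open and shut when its C++ OpenDoor component fires OnOpen or OnClose.
; The DoorSwing timeline plays or reverses, lerping yaw toward the component's OpenAngle and combining it with the rotation saved at BeginPlay.
; Timeline event tracks play creak or slam sounds at the Audio component, using a DoorClosed flag to choose by swing direction.
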(event `self.ReceiveBeginPlay`
  (set `self.Initial Rotation` (`self.K2_GetActorRotation`)))

(event `self.OpenDoor.OnOpen`
  (bind _returnvalue (`SceneComponent.K2_GetComponentLocation` (`self.Audio`)))
  (bind (_direction _open_angle) (`Timeline|Door Swing` :!label _label)
    (:`Update`
      (`self.K2_SetActorRotation` (`KismetMathLibrary.ComposeRotators` (`KismetMathLibrary.RLerp` (struct) (`KismetMathLibrary.MakeRotator` 0.0 0.0 (`OpenDoor.OpenAngle` (`self.OpenDoor`))) _open_angle) (`self.Initial Rotation`))))
    (:`Open Sound Timing`
      (if (`self.Door Closed`)
        (`GameplayStatics.PlaySoundAtLocation` "/Game/Audio/door_creak_short-med_Cue.door_creak_short-med_Cue" _returnvalue)
        (set `self.Door Closed` false)
        (else
          (`GameplayStatics.PlaySoundAtLocation` "/Game/Audio/door_close_slam_slow_Cue.door_close_slam_slow_Cue" _returnvalue)
          (set `self.Door Closed` true))))
    (:`Closed Sound Timing`
      (if (not (`self.Door Closed`))
        (`GameplayStatics.PlaySoundAtLocation` "/Game/Audio/door_creak_short-med_Cue.door_creak_short-med_Cue" _returnvalue)))))

(event `self.OpenDoor.OnClose`
  (goto _label :!via `Reverse`))

(fn `UserConstructionScript`)